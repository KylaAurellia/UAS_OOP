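; BP_Enemy1 is an enemy actor that damages whatever overlaps its capsule, applying a random amount within a fixed range.
; On BeginPlay it finds the BP_EnemySpawner in the level and caches a reference to it.
; After a short delay it increments the spawner's AmountsOfEnemyKilled and calls CheckAmountsOfEnemies, so that count rises on a timer after spawn, independent of any death.
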(event `self.ReceiveTick`
  (params (DeltaSeconds :type "Float (single-precision)")))

(event `self.ReceiveBeginPlay`
  (bind _enemy_spawner (`self.enemy spawner`))
  (bind _returnvalue (`GameplayStatics.GetActorOfClass` "/Game/code/enemy/BP_EnemySpawner.BP_EnemySpawner_C"))
  (set `self.enemy spawner` _returnvalue)
  (`KismetSystemLibrary.Delay` 1.0)
  (`/Engine/EditorBlueprintResources/StandardMacros.IncrementInt` (`/Game/code/enemy/BP_EnemySpawner.amounts of enemy killed` _enemy_spawner)
    (:`  `
      (`/Game/code/enemy/BP_EnemySpawner.check amounts of enemies` _enemy_spawner))))

(event `self.CapsuleComponent.OnComponentBeginOverlap`
  (params (OverlappedComponent :type "PrimitiveComponent Object Reference") (OtherActor :type "Actor Object Reference") (OtherComp :type "PrimitiveComponent Object Reference") (OtherBodyIndex :type Integer) (bFromSweep :type Boolean) (SweepResult :type "HitResult Structure (by ref)"))
  (`GameplayStatics.ApplyDamage` OtherActor (`KismetMathLibrary.RandomFloatInRange` 10.0 25.0) null self))

(fn `UserConstructionScript`)