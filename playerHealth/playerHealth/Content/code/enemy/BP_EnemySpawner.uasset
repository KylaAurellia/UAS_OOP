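; BP_EnemySpawner is an enemy spawner that spawns an AI pawn on a looping timer started at BeginPlay.
; Each tick of the timer picks one of three spawn-location components at random, then rolls for the first or second class in EnemiesToSpawn.
; The range checks use separate random rolls, so some cycles spawn nothing.
; The third enemy branch and a random-offset location calculation are unconnected.
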(event `Sapwn Enemy`
  (bind _returnvalue (`KismetMathLibrary.RandomIntegerInRange` 0 100))
  (switch `int` (`KismetMathLibrary.RandomIntegerInRange` 0 2)
    (:`0`
      (set `self.enemyOn location` (`SceneComponent.K2_GetComponentLocation` (`self.EnemySpawnLocation`))))
    (:`1`
      (set `self.enemyOn location` (`SceneComponent.K2_GetComponentLocation` (`self.EnemySpawnLocation1`))))
    (:`2`
      (set `self.enemyOn location` (`SceneComponent.K2_GetComponentLocation` (`self.EnemySpawnLocation2`)))))
  (if (< _returnvalue 50)
    (`AIBlueprintHelperLibrary.SpawnAIFromClass` (`|GetArrayItem` (`self.enemies to spawn`)) null (`self.enemyOn location`) (struct) false null)
    (elif (and (>= _returnvalue 50) (< _returnvalue 75))
      (`AIBlueprintHelperLibrary.SpawnAIFromClass` (`|GetArrayItem` (`self.enemies to spawn`) 1) null (`self.enemyOn location`) (struct) false null))))

(event `self.ReceiveBeginPlay`
  (`KismetSystemLibrary.K2_SetTimerDelegate` (delegate `Sapwn Enemy`) 5.0 true))

(fn `UserConstructionScript`)