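; BP_ObjectSpawner is an actor that endlessly spawns objects, likely coins, from the start of play.
; Its SpawnCoins event waits a random one to five seconds, then spawns the RandomSpawnObject class at one of five randomly chosen scene component transforms.
; A single-iteration loop then calls the event again, forming a self-repeating delayed cycle.
; An unconnected random-offset location calculation never runs.
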(event `self.ReceiveBeginPlay`
  (`self.Spawn coins`))

(event `Spawn coins`
  (`KismetSystemLibrary.Delay` (`KismetMathLibrary.RandomFloatInRange` 1.0 5.0))
  (for _ (range 1)
    (`|SpawnActorFromClass` "/Game/code/COIN/randomSpawnObject.randomSpawnObject_C" (`SceneComponent.K2_GetComponentToWorld` (select `int` (`KismetMathLibrary.RandomIntegerInRange` 0 4) :`0` (`self.Scene`) :`1` (`self.Scene1`) :`2` (`self.Scene2`) :`3` (`self.Scene3`) :`4` (`self.Scene4`))) "Undefined" "OverrideRootScale" null null)
    (`self.Spawn coins`)))

(fn `UserConstructionScript`)